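; BP_AR4Bullet is the AR4 weapon's bullet projectile, which destroys itself as soon as it reports a hit.
; An unconnected impact sequence remains in the event graph and never runs.
; It would embed the bullet in static surfaces with a timeline-driven roll wiggle, then drop it as a pawn-ignoring physics object before delayed destruction.
; Non-static or invalid hits there would skip straight to the physics drop.
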(event EventOnProjectileHit
  (params (Hit :type Hit%20Result%20Structure%20%28by%20ref%29))
  (Actor|DestroyActor))

(fn ConstructionScript)