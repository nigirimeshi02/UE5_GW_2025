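; Flying bomb enemy Blueprint that blinks with increasing speed while its countdown is active.
; BeginPlay creates a dynamic material on the sphere, and a timeline drives its BlinkColor parameter while IsCountingDown is true.
; Each timeline update raises BlinkRate, which Tick feeds back as the play rate to accelerate the blink.
; When not counting down, Tick moves the weak point sphere far up its relative Z axis, once.
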(event EventBeginPlay
  (bind _returnvalue (Rendering|Material|CreateDynamicMaterialInstance (Variables|Default|GetSphere) 0 "/Game/Enemy/BlinkColor.BlinkColor" "None" :!class /Script/Engine.PrimitiveComponent))
  (Variables|Default|Setmaterial _returnvalue))

(event EventTick
  (params (DeltaSeconds :type Float%20%28single-precision%29))
  (if (Variables|Default|GetbIsCountingDown)
    (Components|Timeline|SetPlayRate (Variables|Default|GetTimeline) (Variables|Default|GetBlinkRate))
    (bind _colortrack (Timeline|Timeline Play)
      (:Update
        (Rendering|Material|SetVectorParameterValue (Variables|Default|Getmaterial) "BlinkColor" _colortrack :!class /Script/Engine.MaterialInstanceDynamic)
        (Variables|Default|SetBlinkRate (+ (Variables|Default|GetBlinkRate) 0.05))))
    (else
      (Utilities|FlowControl|DoOnce false
        (:Completed
          (Transformation|SetRelativeLocation (Variables|Default|GetWeakPointSphere) "0.000000,0.000000,12000.000000" false false))))))

(fn ConstructionScript)