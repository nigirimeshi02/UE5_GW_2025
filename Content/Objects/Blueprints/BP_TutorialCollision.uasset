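; BP_TutorialCollision is a one-shot trigger volume that shows a tutorial tip for a movement or combat action.
; When a GWPlayer overlaps its Box, CheckTextType converts the Preview value into a matching TextType string through nested branches.
; It passes both values to VisibleTips on player 0's BP_GWPlayerController, then destroys itself.
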(event OnComponentBeginOverlap(Box)
  (params (OverlappedComponent :type Primitive%20Component%20Object%20Reference) (OtherActor :type Actor%20Object%20Reference) (OtherComp :type Primitive%20Component%20Object%20Reference) (OtherBodyIndex :type Integer) (bFromSweep :type Boolean) (SweepResult :type Hit%20Result%20Structure%20%28by%20ref%29))
  (Utilities|Casting|CastToGWPlayer OtherActor)
  (bind _asbp_gwplayer_controller (Utilities|Casting|CastToBP_GWPlayerController (Game|GetPlayerController 0)))
  (CallFunction|CheckTextType)
  (Default|VisibleTips _asbp_gwplayer_controller (Variables|Default|GetPreview) (Variables|Default|GetText%20Type))
  (Actor|DestroyActor))

(event EventBeginPlay)

(event Collision|EventActorBeginOverlap
  (params (OtherActor :type Actor%20Object%20Reference)))

(event EventTick
  (params (DeltaSeconds :type Float%20%28single-precision%29)))

(fn ConstructionScript)

(fn CheckTextType
  (if (== (Variables|Default|GetPreview) "/Game/Movies/GrapplingHook.GrapplingHook")
    (Variables|Default|SetText%20Type "GrapplingHook")
    (elif (== (Variables|Default|GetPreview) "/Game/Movies/WallRun.WallRun")
      (Variables|Default|SetText%20Type "WallRun")
      (elif (== (Variables|Default|GetPreview) "/Game/Movies/Climb.Climb")
        (Variables|Default|SetText%20Type "Climb")
        (elif (== (Variables|Default|GetPreview) "/Game/Movies/ADS.ADS")
          (Variables|Default|SetText%20Type "ADS")
          (elif (== (Variables|Default|GetPreview) "/Game/Movies/Fire.Fire")
            (Variables|Default|SetText%20Type "Fire")
            (elif (== (Variables|Default|GetPreview) "/Game/Movies/Reload.Reload")
              (Variables|Default|SetText%20Type "Reload")
              (elif (== (Variables|Default|GetPreview) "/Game/Movies/SwitchWeapon.SwitchWeapon")
                (Variables|Default|SetText%20Type "SwitchWeapon")))))))))