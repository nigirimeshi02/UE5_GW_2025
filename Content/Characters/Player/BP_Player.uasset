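; First-person player character Blueprint that adds a grappling hook and a slide.
; Tick line-traces from the camera to flag CanGrapple, while the grapple input traces again, hops the character, then uses a timeline to extend the wire and move the capsule to the hit.
; A delayed reset restores gravity and the weapon's magazine mesh.
; Sliding plays a montage and timeline-shrinks the capsule; FOV-kick events exist but only unwired nodes call them.
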(event Custom|ShootGrappleHook
  (bind _returnvalue (Class|GWPlayer|GetCurrentWeapon))
  ;[0.15 0.15 0.15 0.5] グラップリングフック
  (Rendering|SetVisibility (Variables|Default|GetGrappleWire) true false)
  (Utilities|IsValid _returnvalue
    (:Is%20Valid
      (Rendering|SetVisibility (Class|ShootingWeapon|GetMagazineMeshComp _returnvalue) false false)
      (bind _interpspeed (Timeline|GrappleTimeline PlayFromStart)
        (:Update
          (Transformation|SetWorldLocation (Variables|Default|GetGrappleWire) (Math|Interpolation|VInterpTo (Transformation|GetWorldLocation (Variables|Default|GetGrappleWire)) (Variables|グラップリングフック|GetGrapplePoint) (Utilities|Time|GetWorldDeltaSeconds) _interpspeed) false true)
          (Components|MoveComponentTo (Variables|Default|GetCapsuleComponent) (Variables|グラップリングフック|GetGrapplePoint) "0, 0, 0" false false 0.2 false :!label _label))
        (:Finished
          (goto _label Stop))))
    (:Is%20Not%20Valid
      (Timeline|GrappleTimeline PlayFromStart))))

(event Custom|ResetGrappleHook
  (bind _returnvalue (Class|GWPlayer|GetCurrentWeapon))
  ;[0.15 0.15 0.15 0.5] グラップリングフック
  (Rendering|SetVisibility (Variables|Default|GetGrappleWire) false false)
  (Utilities|IsValid _returnvalue
    (:Is%20Valid
      (Rendering|SetVisibility (Class|ShootingWeapon|GetMagazineMeshComp _returnvalue) true false)
      (Variables|/Script/Engine.CharacterMovementComponent|SetGravityScale (Variables|Character|GetCharacterMovement) (Variables|グラップリングフック|GetGravity))
      (Variables|グラップリングフック|SetIsGrapple false))))

(event Custom|StopFOV
  (bind _fieldofview (Variables|FOV|GetFieldOfView))
  ;[0.15 0.15 0.15 0.5] グラップリングフック
  (if (Variables|FOV|GetIsApplendFOV)
    (bind (_direction _alpha) (Timeline|FOVTimeline Reverse)
      (:Update
        (Camera|SetFieldOfView (Variables|Default|GetFirstPersonCameraComponent) (Math|Float|Lerp _fieldofview (+ _fieldofview 2e+01) _alpha)))
      (:Finished
        (if (Utilities|Enum|Equal(Enum) _direction "Backward")
          (Variables|FOV|SetIsApplendFOV false))))))

(event Custom|StartFOV
  ;[0.15 0.15 0.15 0.5] グラップリングフック
  (if (not (Variables|FOV|GetIsApplendFOV))
    (Variables|FOV|SetIsApplendFOV true)
    (Variables|FOV|SetFieldOfView (Variables|/Script/Engine.CameraComponent|GetFieldOfView (Variables|Default|GetFirstPersonCameraComponent)))
    (bind (_direction _alpha) (Timeline|FOVTimeline Play)
      (:Update
        (Camera|SetFieldOfView (Variables|Default|GetFirstPersonCameraComponent) (Math|Float|Lerp (Variables|FOV|GetFieldOfView) (+ (Variables|FOV|GetFieldOfView) 2e+01) _alpha)))
      (:Finished
        (if (Utilities|Enum|Equal(Enum) _direction "Backward")
          (Variables|FOV|SetIsApplendFOV false))))))

(event Input|EnhancedActionEvents|EnhancedInputActionIA_Slide
  (params (ActionValue :type Boolean) (ElapsedSeconds :type Float%20%28double-precision%29) (TriggeredSeconds :type Float%20%28double-precision%29) (InputAction :type Input%20Action%20Object%20Reference :default "/Game/Input/Actions/IA_Slide.IA_Slide"))
  ;[0.15 0.15 0.15 0.5] スライディング
  (:Started
    (if (not (AI|Components|NavMovement|IsFalling (Variables|Character|GetCharacterMovement)))
      (if (not (Variables|Default|GetIsSlide))
        (Variables|Default|SetIsSlide true)
        (Animation|Montage|PlayMontage (Variables|Character|GetMesh) "/Game/Characters/Player/Animations/RunningSlide_UE_Montage.RunningSlide_UE_Montage" 1.2
          (:then
            (bind (_direction _slider) (Timeline|SlideTimeline PlayFromStart)
              (:Update
                (switch Utilities|FlowControl|Switch|SwitchonETimelineDirection _direction
                  (:Forward
                    (Components|Capsule|SetCapsuleHalfHeight (Variables|Default|GetCapsuleComponent) (Math|Float|Lerp 96.0 3e+01 _slider) true))
                  (:Backward
                    (Components|Capsule|SetCapsuleHalfHeight (Variables|Default|GetCapsuleComponent) (Math|Float|Lerp 96.0 3e+01 _slider) true))))))
          (:OnCompleted
            (Variables|Default|SetIsSlide false :!label _label)
            (Timeline|SlideTimeline Reverse))
          (:OnInterrupted
            (goto _label)))))))

(event Input|EnhancedActionEvents|EnhancedInputActionIA_GrapplingHook
  (params (ActionValue :type Boolean) (ElapsedSeconds :type Float%20%28double-precision%29) (TriggeredSeconds :type Float%20%28double-precision%29) (InputAction :type Input%20Action%20Object%20Reference :default "/Game/Input/Actions/IA_GrapplingHook.IA_GrapplingHook"))
  (bind _firstpersoncameracomponent (Variables|Default|GetFirstPersonCameraComponent))
  (bind _returnvalue (Transformation|GetWorldLocation _firstpersoncameracomponent))
  ;[0.15 0.15 0.15 0.5] グラップリングフック
  (:Started
    (if (not (Variables|グラップリングフック|GetIsGrapple))
      (Variables|グラップリングフック|SetIsGrapple true) ; グラップル中
      (Variables|/Script/Engine.CharacterMovementComponent|SetGravityScale (Variables|Character|GetCharacterMovement) 1.0)
      (bind (_outhit _returnvalue_2) (Collision|LineTraceByChannel _returnvalue (+ _returnvalue (* (Math|Vector|GetForwardVector _firstpersoncameracomponent) (Variables|グラップリングフック|GetGrappleLength))) "TraceTypeQuery3" false 0 "None"))
      (if _returnvalue_2
        (Variables|グラップリングフック|SetGrapplePoint (.ImpactPoint (Collision|BreakHitResult _outhit))) ; 掴んでいる場所
        (CallFunction|ShootGrappleHook)
        (Character|LaunchCharacter "0.000000,0.000000,100.000000" true true)
        (Audio|PlaySoundatLocation "/Game/Sound/Free_Sounds_Pack/wav/Sci-Fi_Gun_1_Reload.Sci-Fi_Gun_1_Reload" "0, 0, 0" "0, 0, 0" 1.0 1.0 0.0 0 0 0 0)
        (Utilities|FlowControl|Delay 0.4)
        (CallFunction|ResetGrappleHook)
        (else
          (CallFunction|ResetGrappleHook))))))

(event EventTick
  (params (DeltaSeconds :type Float%20%28single-precision%29))
  (bind _firstpersoncameracomponent (Variables|Default|GetFirstPersonCameraComponent))
  (bind _returnvalue (Transformation|GetWorldLocation _firstpersoncameracomponent))
  (bind _returnvalue_2 (Collision|LineTraceByChannel _returnvalue (+ _returnvalue (* (Math|Vector|GetForwardVector _firstpersoncameracomponent) (Variables|グラップリングフック|GetGrappleLength))) "TraceTypeQuery3" false 0 "None" true "(R=1.000000,G=0.000000,B=0.000000,A=1.000000)" "(R=0.000000,G=1.000000,B=0.000000,A=1.000000)" 1.0))
  (if _returnvalue_2
    (Variables|グラップリングフック|SetCanGrapple true)
    (else
      (Variables|グラップリングフック|SetCanGrapple false))))

(event EventBeginPlay
  (Class|MovementComponent|SetPlaneConstraintEnabled (Variables|Character|GetCharacterMovement) true)
  (Variables|グラップリングフック|SetGravity (Variables|/Script/Engine.CharacterMovementComponent|GetGravityScale (Variables|Character|GetCharacterMovement))))

(fn ConstructionScript)